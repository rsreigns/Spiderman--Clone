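; Quest manager that tracks objective progress across day and night shifts and shows the current quest on screen.
; On BeginPlay it creates the quest widget and loads saved progress from the GameInstance.
; Finished objectives advance the ID, flipping shift and incrementing the day (capped) past each shift's task limit, then refresh UI from per-shift DataTables and save to the GameInstance.
; ShowQuest, StartNextQuest and the shift-finished events are empty stubs.
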(event `self.ReceiveBeginPlay`
  (bind _returnvalue (`|CreateWidget` "/Game/QuestSystem/UI/WBP_Quest.WBP_Quest_C" (`GameplayStatics.GetPlayerController` 0)))
  (set `self.QuestWidget` _returnvalue)
  (bind _savedgamedata (message `/Game/QuestSystem/Interfaces/Quest_Interface.LoadSavedGame` (`GameplayStatics.GetGameInstance`)))
  (set `self.QuestData` _savedgamedata)
  (`self.UpdateQuestUI`)
  (`UserWidget.AddToViewport` (`self.QuestWidget`) 0))

(event `/Game/QuestSystem/Interfaces/Quest_Interface.ShowQuest`
  (params (bShouldShowQuest :type Boolean))
  (if bShouldShowQuest
    _))

(event `/Game/QuestSystem/Interfaces/Quest_Interface.NightShiftFinished`)

(event `/Game/QuestSystem/Interfaces/Quest_Interface.DayObjectiveFinished`)

(event `/Game/QuestSystem/Interfaces/Quest_Interface.ObjectiveFinished`
  (params (HasFinishedQuest :type Boolean))
  (bind (_currentday _currentshift _currentobjective_id) (break `/Game/QuestSystem/Structures/FQuestTrack` (`self.QuestData`)))
  (bind _returnvalue (`KismetStringLibrary.Conv_StringToName` (`KismetStringLibrary.Conv_IntToString` _currentobjective_id)))
  (if HasFinishedQuest
    (set `self.QuestData` (`self.CalculateCurrentObjective`))
    (switch `/Game/QuestSystem/Enum/E_DayShift` _currentshift
      (:`NewEnumerator0`
        (bind _returnvalue_2 (`|GetDataTableRow` "/Game/QuestSystem/DataTables/DT_QuestData_Day.DT_QuestData_Day" _returnvalue)
          (:`then`
            (set `self.Out Row` _returnvalue_2))))
      (:`NewEnumerator1`
        (bind _returnvalue_3 (`|GetDataTableRow` "/Game/QuestSystem/DataTables/DT_QuestData_Night.DT_QuestData_Night" _returnvalue)
          (:`then`
            (set `self.Out Row` _returnvalue_3)))))
    (`self.UpdateQuestUI`)
    (message `/Game/QuestSystem/Interfaces/Quest_Interface.SaveQuestToGameInstance` (`GameplayStatics.GetGameInstance`) (`self.QuestData`))))

(fn `CalculateCurrentObjective`
  (returns (FQuestTrack :type "/Game/QuestSystem/Structures/FQuestTrack Structure"))
  (locals (FinalData :type "/Game/QuestSystem/Structures/FQuestTrack Structure"))
  (bind (_currentday _currentshift _currentobjective_id) (break `/Game/QuestSystem/Structures/FQuestTrack` (`self.QuestData`)))
  (bind (_currentday_2 _currentshift_2 _currentobjective_id_2) (break `/Game/QuestSystem/Structures/FQuestTrack` (`self.QuestData`)))
  (bind _returnvalue (+ _currentobjective_id_2 1))
  (bind _returnvalue_2 (+ _currentday_2 1))
  (bind _returnvalue_3 (+ _currentobjective_id 1))
  (bind _returnvalue_4 (+ _currentday 1))
  (bind _returnvalue_5 (and (`|EnumEquality` _currentshift_2 "NewEnumerator1") (> _returnvalue (`self.MaxNightTasks`))))
  (bind _returnvalue_6 (and (`|EnumEquality` _currentshift "NewEnumerator0") (> _returnvalue_3 (`self.MaxDayTasks`))))
  (switch `/Game/QuestSystem/Enum/E_DayShift` (`.CurrentShift_9_679111AD468A1A793F10A6BE94FA775C` (break `/Game/QuestSystem/Structures/FQuestTrack` (`self.QuestData`)))
    (:`NewEnumerator0`
      (set `local.FinalData` (make `/Game/QuestSystem/Structures/FQuestTrack` (select `bool` (and _returnvalue_6 (<= _returnvalue_4 (`self.MaxDays`))) :`false` _currentday :`true` _returnvalue_4) (select `bool` _returnvalue_6 :`false` "NewEnumerator0" :`true` "NewEnumerator1" :!type "/Game/QuestSystem/Enum/E_DayShift Enum") (`KismetMathLibrary.SelectInt` 1 _returnvalue_3 _returnvalue_6))))
    (:`NewEnumerator1`
      (set `local.FinalData` (make `/Game/QuestSystem/Structures/FQuestTrack` (select `bool` (and _returnvalue_5 (<= _returnvalue_2 (`self.MaxDays`))) :`false` _currentday_2 :`true` _returnvalue_2) (select `bool` _returnvalue_5 :`false` "NewEnumerator1" :`true` "NewEnumerator0" :!type "/Game/QuestSystem/Enum/E_DayShift Enum") (`KismetMathLibrary.SelectInt` 1 _returnvalue _returnvalue_5)))))
  (return (`local.FinalData`)))

(fn `LoadSavedGame`
  (returns (SavedGameData :type "/Game/QuestSystem/Structures/FQuestTrack Structure"))
  (return))

(fn `StartNextQuest`
  (params (PrevQuestNum :type Integer64)))

(fn `UpdateQuestUI`
  (locals (UpdatedObjData :type "/Game/QuestSystem/Structures/FRow_QuestTable Structure"))
  (bind (_questdata_currentday _questdata_currentshift _questdata_currentobjective_id) (break `/Game/QuestSystem/Structures/FQuestTrack` (`self.QuestData`)))
  (bind _returnvalue (`KismetStringLibrary.Conv_StringToName` (`KismetStringLibrary.Conv_IntToString` _questdata_currentobjective_id)))
  (switch `/Game/QuestSystem/Enum/E_DayShift` _questdata_currentshift
    (:`NewEnumerator0`
      (bind _returnvalue_2 (`|GetDataTableRow` "/Game/QuestSystem/DataTables/DT_QuestData_Day.DT_QuestData_Day" _returnvalue)
        (:`then`
          (message `/Game/QuestSystem/Interfaces/Quest_Interface.UpdateUI` (`self.QuestWidget`) (`KismetStringLibrary.Conv_IntToString` (break `/Game/QuestSystem/Structures/FRow_QuestTable` _returnvalue_2)) (`.QuestTitle_6_6756675A4FACD7DCE0812695D1D33D41` (break `/Game/QuestSystem/Structures/FRow_QuestTable` _returnvalue_2)) (`.QuestDescription_9_0424CBC6400E7D0660915B96B9895CD2` (break `/Game/QuestSystem/Structures/FRow_QuestTable` _returnvalue_2))))))
    (:`NewEnumerator1`
      (bind _returnvalue_3 (`|GetDataTableRow` "/Game/QuestSystem/DataTables/DT_QuestData_Night.DT_QuestData_Night" _returnvalue)
        (:`then`
          (message `/Game/QuestSystem/Interfaces/Quest_Interface.UpdateUI` (`self.QuestWidget`) (`KismetStringLibrary.Conv_IntToString` (break `/Game/QuestSystem/Structures/FRow_QuestTable` _returnvalue_3)) (`.QuestTitle_6_6756675A4FACD7DCE0812695D1D33D41` (break `/Game/QuestSystem/Structures/FRow_QuestTable` _returnvalue_3)) (`.QuestDescription_9_0424CBC6400E7D0660915B96B9895CD2` (break `/Game/QuestSystem/Structures/FRow_QuestTable` _returnvalue_3))))))))