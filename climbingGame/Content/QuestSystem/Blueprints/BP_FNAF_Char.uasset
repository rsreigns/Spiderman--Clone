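; BP_FNAF_Char is a player character in the quest system with Enhanced Input movement, camera look and interaction.
; While flagged in interaction range, Tick traces along the camera's forward vector, caching the hit actor and whether it implements Quest_Interface.
; IA_Interact sends PressedInteractMessage to that actor when CanInteract is true.
; CanInteract updates only when a trace hits, and LoadSavedGame is an empty stub.
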(event `self.ReceiveBeginPlay`
  (bind _asplayer_controller (cast `PlayerController` (`self.GetController`)))
  (`EnhancedInputSubsystemInterface.AddMappingContext` (pcsubsystem `EnhancedInputLocalPlayerSubsystem` _asplayer_controller) "/Game/QuestSystem/Input/IMC_Quest_Default.IMC_Quest_Default" 0 (struct)))

(event `EnhancedInput|/Game/QuestSystem/Input/Actions/IA_Move`
  (params (ActionValue :type "Vector2D Structure") (ElapsedSeconds :type "Float (double-precision)") (TriggeredSeconds :type "Float (double-precision)") (InputAction :type "InputAction Object Reference" :default "/Game/QuestSystem/Input/Actions/IA_Move.IA_Move"))
  (:`Triggered`
    (`self.AddMovementInput` (`SceneComponent.GetForwardVector` (`self.Camera`)) ActionValue_Y)
    (`self.AddMovementInput` (`SceneComponent.GetRightVector` (`self.Camera`)) ActionValue_X)))

(event `EnhancedInput|/Game/QuestSystem/Input/Actions/IA_Look`
  (params (ActionValue :type "Vector2D Structure") (ElapsedSeconds :type "Float (double-precision)") (TriggeredSeconds :type "Float (double-precision)") (InputAction :type "InputAction Object Reference" :default "/Game/QuestSystem/Input/Actions/IA_Look.IA_Look"))
  (:`Triggered`
    (`self.AddControllerPitchInput` ActionValue_Y)
    (`self.AddControllerYawInput` ActionValue_X)))

(event `/Game/QuestSystem/Interfaces/Quest_Interface.InInteractionRange`
  (params (bInRange :type Boolean))
  (set `self.bIsInInteractRange` bInRange))

(event `EnhancedInput|/Game/QuestSystem/Input/Actions/IA_Interact`
  (params (ActionValue :type Boolean) (ElapsedSeconds :type "Float (double-precision)") (TriggeredSeconds :type "Float (double-precision)") (InputAction :type "InputAction Object Reference" :default "/Game/QuestSystem/Input/Actions/IA_Interact.IA_Interact"))
  (:`Started`
    (if (`self.bCanInteract`)
      (message `/Game/QuestSystem/Interfaces/Quest_Interface.PressedInteract` (`self.LineTraceHitActor`)))))

(event `self.ReceiveTick`
  (params (DeltaSeconds :type "Float (single-precision)"))
  (if (`self.bIsInInteractRange`)
    (`self.TraceForInteraction`)))

(fn `LineTrace`
  (params (Start :type "Vector Structure") (End :type "Vector Structure") (DrawDebugType :type "EDrawDebugTrace Enum" :default "None"))
  (returns (OutHit :type "HitResult Structure") (ReturnValue :type Boolean))
  (bind (_outhit _returnvalue) (`KismetSystemLibrary.LineTraceSingle` Start End "TraceTypeQuery1" false (`|MakeArray` self :!type "Actor Object Reference") DrawDebugType))
  (bind (_bblockinghit _binitialoverlap _time _distance _location _impactpoint _normal _impactnormal _physmat _hitactor _hitcomponent) (`GameplayStatics.BreakHitResult` _outhit))
  (set `self.LineTraceHitActor` _hitactor)
  (set `self.LineTraceHitComponent` _hitcomponent)
  (return _outhit _returnvalue))

(fn `LoadSavedGame`
  (returns (SavedGameData :type "/Game/QuestSystem/Structures/FQuestTrack Structure"))
  (return))

(fn `TraceForInteraction`
  (bind _camera (`self.Camera`))
  (bind _returnvalue (`SceneComponent.K2_GetComponentLocation` _camera))
  (bind (_outhit _returnvalue_2) (`self.LineTrace` _returnvalue (+ _returnvalue (* (`SceneComponent.GetForwardVector` _camera) (`self.InteractionRange`)))))
  (if _returnvalue_2
    (set `self.bCanInteract` (`KismetSystemLibrary.DoesImplementInterface` (`self.LineTraceHitActor`) "/Game/QuestSystem/Interfaces/Quest_Interface.Quest_Interface_C"))
    (return)))

(fn `UserConstructionScript`)