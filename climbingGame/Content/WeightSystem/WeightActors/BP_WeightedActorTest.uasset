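; BP_WeightedActorTest is a test actor for the weight system, pairing a Cube mesh with a BPWeightComponent.
; The construction script sets the Cube's mass scale from the component's ObjectWeight.
; Hit events are forwarded to the component's HandleHitEvent, followed by a debug print.
; Logic for notifying the component when an object above moves away and a debug sphere draw are disconnected, and Box end-overlap is empty.
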(event `self.ReceiveBeginPlay`)

(event `self.ReceiveTick`
  (params (DeltaSeconds :type "Float (single-precision)")))

(event `self.Box.OnComponentEndOverlap`
  (params (OverlappedComponent :type "PrimitiveComponent Object Reference") (OtherActor :type "Actor Object Reference") (OtherComp :type "PrimitiveComponent Object Reference") (OtherBodyIndex :type Integer)))

(event `self.ReceiveHit`
  (params (MyComp :type "PrimitiveComponent Object Reference") (Other :type "Actor Object Reference") (OtherComp :type "PrimitiveComponent Object Reference") (bSelfMoved :type Boolean) (HitLocation :type "Vector Structure") (HitNormal :type "Vector Structure") (NormalImpulse :type "Vector Structure") (Hit :type "HitResult Structure (by ref)"))
  (`WeightComponent.HandleHitEvent` (`self.BP_WeightComponent`) Other)
  (`KismetSystemLibrary.PrintString` "Hello" true true (struct :`G` 0.66 :`B` 1.0 :`A` 1.0) 0.0))

(fn `UserConstructionScript`
  (`PrimitiveComponent.SetMassScale` (`self.Cube`) "None" (`WeightComponent.ObjectWeight` (`self.BP_WeightComponent`))))