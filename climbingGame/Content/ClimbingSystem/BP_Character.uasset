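; Player character with sprinting, wall running, dashing and web swinging, using a custom movement component.
; Sprinting swaps to a first-person camera; Tick sphere-traces for walls, then plane-constrains and launches the character along the camera direction.
; During wall contact, Space plays a montage motion-warped to a camera line-trace point.
; Clicking mid-air places a constraint SwingBox and physics-simulates the capsule under input forces; releasing breaks the constraint, while hits during swings restore pawn collision.
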(event `Key|LeftShift`
  (params (Key :type "Key Structure"))
  (bind _fp_cam (`self.FP_Cam`))
  (bind _followcamera (`self.FollowCamera`))
  (bind _cameraboom (`self.CameraBoom`))
  (bind _fp_camarm (`self.FP_CamArm`))
  (bind _custommovementcomponent (`self.CustomMovementComponent`))
  (bind _returnvalue (`|EnumInequality` (`CharacterMovementComponent.MovementMode` (`self.CustomMovementComponent`)) "MOVE_Custom"))
  ;[0 0 0] Sprint + First Person Cam
  (:`Pressed`
    (if _returnvalue
      (set `CharacterMovementComponent.MaxWalkSpeed` 600.0 _custommovementcomponent)
      (set `self.bIsSprinting` true)
      (`ActorComponent.SetActive` _fp_cam true false)
      (`ActorComponent.SetActive` _followcamera false false)
      (`ActorComponent.SetActive` _cameraboom false false)
      (set `SpringArmComponent.bUsePawnControlRotation` false _cameraboom)
      (`ActorComponent.SetActive` _fp_camarm true false)
      (set `SpringArmComponent.bUsePawnControlRotation` true _fp_camarm)
      (set `self.bUseControllerRotationYaw` true)))
  (:`Released`
    (if _returnvalue
      (set `CharacterMovementComponent.MaxWalkSpeed` 300.0 _custommovementcomponent)
      (set `self.bIsSprinting` false)
      (`ActorComponent.SetActive` _fp_cam false false)
      (`ActorComponent.SetActive` _followcamera true false)
      (`ActorComponent.SetActive` _cameraboom true false)
      (set `SpringArmComponent.bUsePawnControlRotation` true _cameraboom)
      (`ActorComponent.SetActive` _fp_camarm false false)
      (set `SpringArmComponent.bUsePawnControlRotation` false _fp_camarm)
      (set `self.bUseControllerRotationYaw` false))))

(event `Key|LeftAlt`
  (params (Key :type "Key Structure"))
  (bind _custommovementcomponent (`self.CustomMovementComponent`))
  (:`Pressed`
    (if (`NavMovementComponent.IsFalling` (`self.CustomMovementComponent`))
      (set `CharacterMovementComponent.GravityScale` 10.0 _custommovementcomponent)
      (else
        (set `CharacterMovementComponent.GravityScale` 1.0 _custommovementcomponent)))))

(event `Key|SpaceBar`
  (params (Key :type "Key Structure"))
  ;[0 0 0] Launch player
  (:`Pressed`
    (if (`self.bShouldWallRun`)
      (bind (_outhit _location) (`self.LineTraceFrontCam`))
      (`MotionWarpingComponent.AddOrUpdateWarpTargetFromLocation` (`self.MotionWarpingComponent`) "DashToLocation" _location)
      (`MovementComponent.SetPlaneConstraintEnabled` (`self.CharacterMovement`) false)
      (set `self.bCanWallRun` false)
      (`|PlayMontage` (`self.Mesh`) "/Game/ClimbingSystem/Animation/Anim-Assets/Montages/MM_DashToLocation_Montage.MM_DashToLocation_Montage"
        (:`OnCompleted`
          _)
        (:`OnBlendOut`
          _))
      (`MovementComponent.SetPlaneConstraintEnabled` (`self.CharacterMovement`) true)
      (set `self.bCanWallRun` true))))

(event `Key|LeftMouseButton`
  (params (Key :type "Key Structure"))
  (bind _swingbox (`self.SwingBox`))
  (bind _swingbox_2 (`self.SwingBox`))
  (bind _capsulecomponent (`self.CapsuleComponent`))
  (bind (_returnvalue_x _returnvalue_y) (`KismetMathLibrary.BreakVector` (`SceneComponent.GetForwardVector` (`self.FollowCamera`))))
  (bind (_returnvalue_roll _returnvalue_pitch _returnvalue_yaw) (`KismetMathLibrary.BreakRotator` (`SceneComponent.K2_GetComponentRotation` _capsulecomponent)))
  (bind _returnvalue (+ (`self.K2_GetActorLocation`) (* (`KismetMathLibrary.MakeVector` _returnvalue_x _returnvalue_y) (`self.SwingWebForwardDistance`)) (* (0.0 0.0 1.0) (`self.SwingWebLength`))))
  ;[0 0 0] Swinging
  (:`Pressed`
    (if (`NavMovementComponent.IsFalling` (`self.CustomMovementComponent`))
      (`/Engine/EditorBlueprintResources/StandardMacros.IsValid` (`self.SwingBox`)
        (:`Is Valid`
          (`self.K2_SetActorLocation` _swingbox _returnvalue false true)
          (`/Game/ClimbingSystem/Actors/A_SwingBox.setConstraint` _swingbox))
        (:`Is Not Valid`
          (bind _returnvalue_2 (`|SpawnActorFromClass` "/Game/ClimbingSystem/Actors/A_SwingBox.A_SwingBox_C" (`KismetMathLibrary.MakeTransform` _returnvalue) "AdjustIfPossibleButAlwaysSpawn" "MultiplyWithRoot" null self))
          (set `self.SwingBox` _returnvalue_2)))
      (set `self.TargetPivotLocation` _returnvalue)
      (set `self.bIsSwingng` true)
      (`PrimitiveComponent.SetCollisionProfileName` (`self.CapsuleComponent`) "PhysicsActor" true)
      (`PrimitiveComponent.SetSimulatePhysics` (`self.CapsuleComponent`) true)
      (set `self.bUseControllerRotationYaw` false)))
  (:`Released`
    (set `self.bIsSwingng` false)
    (`/Engine/EditorBlueprintResources/StandardMacros.IsValid` _swingbox_2
      (:`Is Valid`
        (`/Game/ClimbingSystem/Actors/A_SwingBox.breakConstraint` _swingbox_2))
      (:`Is Not Valid`
        _))
    (`SceneComponent.K2_SetWorldRotation` _capsulecomponent (`KismetMathLibrary.MakeRotator` 0.0 0.0 _returnvalue_yaw) true false)))

(event `self.ReceiveTick`
  (params (DeltaSeconds :type "Float (single-precision)"))
  (bind (_returnvalue_x _returnvalue_y) (`KismetMathLibrary.BreakVector2D` (`|GetInputActionValue`)))
  (bind (_returnvalue_x_2 _returnvalue_y_2) (`KismetMathLibrary.BreakVector2D` (`|GetInputActionValue`)))
  (bind (_returnvalue_x_3 _returnvalue_y_3) (`KismetMathLibrary.BreakVector2D` (`|GetInputActionValue`)))
  ;[0 0 0] WallRUnning
  (`|ExecutionSequence`
    (:`then_0`
      (if (`|EnumInequality` (`CharacterMovementComponent.MovementMode` (`self.CustomMovementComponent`)) "MOVE_Custom")
        (if (`self.bIsSwingng`)
          ;[0 0 0] Handle Swing movement
          (`PrimitiveComponent.AddForce` (`self.CapsuleComponent`) (* (+ (* (`self.GetActorForwardVector`) _returnvalue_y_2) (* (`self.GetActorRightVector`) _returnvalue_x_2)) (`self.SwingingSpeed`)) "None" true)
          (elif (`self.bIsSprinting`)
            (bind _outhit (`self.SphereTraceAroundPlayer` "ForOneFrame"))
            (bind (_bblockinghit _binitialoverlap _time _distance _location _impactpoint _normal) (`GameplayStatics.BreakHitResult` _outhit))
            (set `self.bShouldWallRun` _bblockinghit)
            (set `self.Normal` _normal)
            (if (`self.bCanWallRun`)
              (`MovementComponent.SetPlaneConstraintEnabled` (`self.CustomMovementComponent`) _bblockinghit)
              (if _bblockinghit
                (if (> _returnvalue_y 0.0)
                  (`MovementComponent.SetPlaneConstraintNormal` (`self.CharacterMovement`) (`self.Normal`))
                  (`self.LaunchCharacter` (* (`SceneComponent.GetForwardVector` (`self.FP_Cam`)) (`self.WallRunningSpeed`) _returnvalue_y_3) true true))))
            (else
              (`MovementComponent.SetPlaneConstraintEnabled` (`self.CustomMovementComponent`) false))))))))

(event `self.ReceiveHit`
  (params (MyComp :type "PrimitiveComponent Object Reference") (Other :type "Actor Object Reference") (OtherComp :type "PrimitiveComponent Object Reference") (bSelfMoved :type Boolean) (HitLocation :type "Vector Structure") (HitNormal :type "Vector Structure") (NormalImpulse :type "Vector Structure") (Hit :type "HitResult Structure (by ref)")))

(event `ReleaseWeb`
  (bind _capsulecomponent (`self.CapsuleComponent`))
  ;[0 0 0] Swinging
  (`PrimitiveComponent.SetCollisionProfileName` _capsulecomponent "Pawn" true)
  (set `self.bUseControllerRotationYaw` false)
  (`PrimitiveComponent.SetSimulatePhysics` _capsulecomponent false)
  (set `self.bIsSwingng` false)
  (`PrimitiveComponent.SetCollisionEnabled` (`self.Mesh`) "QueryOnly"))

(event `self.CapsuleComponent.OnComponentHit`
  (params (HitComponent :type "PrimitiveComponent Object Reference") (OtherActor :type "Actor Object Reference") (OtherComp :type "PrimitiveComponent Object Reference") (NormalImpulse :type "Vector Structure") (Hit :type "HitResult Structure (by ref)"))
  (if (`self.bIsSwingng`)
    (`self.ReleaseWeb`)
    (`KismetSystemLibrary.PrintString` "Released")))

(fn `LineTraceFrontCam`
  (returns (OutHit :type "HitResult Structure") (Location :type "Vector Structure"))
  (bind _fp_cam (`self.FP_Cam`))
  (bind _returnvalue (`SceneComponent.K2_GetComponentLocation` _fp_cam))
  (bind _outhit (`KismetSystemLibrary.LineTraceSingle` :`Start` _returnvalue :`End` (+ _returnvalue (* (`SceneComponent.GetForwardVector` _fp_cam) 2000.0)) :`TraceChannel` "TraceTypeQuery1" :`DrawDebugType` "ForDuration" :`DrawTime` 11.0))
  (bind (_bblockinghit _binitialoverlap _time _distance _location _impactpoint _normal _impactnormal _physmat _hitactor _hitcomponent _hitbonename _bonename _hititem _elementindex _faceindex _tracestart _traceend) (`GameplayStatics.BreakHitResult` _outhit))
  (return _outhit (`KismetMathLibrary.SelectVector` _traceend _impactpoint (`KismetMathLibrary.Vector_IsNearlyZero` _impactpoint))))

(fn `SphereTraceAroundPlayer`
  (params (DrawDebugType :type "EDrawDebugTrace Enum" :default "None"))
  (returns (OutHit :type "HitResult Structure"))
  (bind _returnvalue (`self.K2_GetActorLocation`))
  (bind _returnvalue_2 (* (`self.GetActorUpVector`) 90.0))
  (bind _outhit (`KismetSystemLibrary.SphereTraceSingle` :`Start` (+ (* (`self.GetActorForwardVector`) -30.0) _returnvalue _returnvalue_2) :`End` (+ _returnvalue _returnvalue_2 (* (`self.GetActorForwardVector`) 90.0)) :`Radius` 90.0 :`TraceChannel` "TraceTypeQuery1" :`DrawDebugType` DrawDebugType))
  (return _outhit))

(fn `UserConstructionScript`)